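; Parent Character Blueprint for selectable units that can be ordered to move to a location.
; Selection and deselection events toggle the visibility of a decal on the character.
; The move command event stops the AI controller's current movement, then starts an AI Move To toward the given location.
; BeginPlay, the construction script and GrabSelectedUnits are empty.
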(event `self.ReceiveBeginPlay`)

(event `/Game/Character_Events_INT.Character Selected`
  ;[1 1 1] When character is selected, set decal active, if deselected, disable decal
  (`SceneComponent.SetVisibility` (`self.Decal`) true false))

(event `/Game/Character_Events_INT.Character Deselected`
  ;[1 1 1] When character is selected, set decal active, if deselected, disable decal
  (`SceneComponent.SetVisibility` (`self.Decal`) false false))

(event `/Game/Character_Events_INT.Character Move Command`
  (params (Location :type "Vector Structure"))
  (bind _returnvalue (`AIBlueprintHelperLibrary.GetAIController` self))
  (`Controller.StopMovement` _returnvalue)
  (`AITask_MoveTo.AIMoveTo` _returnvalue Location null))

(fn `Grab Selected Units`
  (returns (`Selected Units` :type "Array of Actor Object Reference"))
  (return))

(fn `UserConstructionScript`)